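; Player character Blueprint that handles the fail, revive and victory moments of play.
; Failing hides the character and weapon and opens a fail menu with UI-only input and cursor.
; Revive restores visibility, walking, full health and game input, then removes the stored fail menu and unhides the weapon if that menu exists.
; Victory shows its menu after a short delay with the same UI input setup.
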(event `self.BP_ShowFailUI`
  (bind _returnvalue (`GameplayStatics.GetPlayerController` 0))
  (`self.SetActorHiddenInGame` true)
  (bind _returnvalue_2 (`|CreateWidget` "/Game/Blueprint/UI/WBP_FailMenu.WBP_FailMenu_C"))
  (set `self.FailWidget` _returnvalue_2)
  (`UserWidget.AddToViewport` _returnvalue_2 0)
  (`WidgetBlueprintLibrary.SetInputMode_UIOnlyEx` _returnvalue null)
  (set `PlayerController.bShowMouseCursor` true _returnvalue)
  (`self.SetActorHiddenInGame` (`self.CurrentWeapon`) true))

(event `Revive`
  (bind _healthcomp (`CharacterBased.HealthComp`))
  (`self.SetActorHiddenInGame` self false)
  (`CharacterMovementComponent.SetMovementMode` (`Character.CharacterMovement`) "MOVE_Walking" 0)
  (`HealthComponent.Heal` _healthcomp (`HealthComponent.MaxHP` _healthcomp))
  (bind _asbp_player_controller (cast `/Game/Blueprint/BP_PlayerController` (`GameplayStatics.GetPlayerController` 0)))
  (`WidgetBlueprintLibrary.SetInputMode_GameOnly` _asbp_player_controller)
  (set `PlayerController.bShowMouseCursor` false _asbp_player_controller)
  (bind _failwidget (`self.FailWidget`)
    (:`then`
      (`Widget.RemoveFromParent` _failwidget)
      (`self.SetActorHiddenInGame` (`self.CurrentWeapon`) false))
    (:`else`)))

(event `self.BP_ShowVictoryUI`
  (bind _returnvalue (`GameplayStatics.GetPlayerController` 0))
  (`KismetSystemLibrary.Delay` 3.0)
  (bind _returnvalue_2 (`|CreateWidget` "/Game/Blueprint/UI/WBP_VectoryMenu.WBP_VectoryMenu_C"))
  (`UserWidget.AddToViewport` _returnvalue_2 0)
  (`WidgetBlueprintLibrary.SetInputMode_UIOnlyEx` _returnvalue null)
  (set `PlayerController.bShowMouseCursor` true _returnvalue))

(fn `UserConstructionScript`)