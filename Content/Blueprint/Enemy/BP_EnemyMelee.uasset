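; Melee enemy character Blueprint that attacks the player with left and right hit boxes.
; DoMeleeAttack plays the melee montage from a randomly chosen section, and OnEnemyDead plays a non-looping death animation on the mesh.
; Hit box overlaps apply AttackDamage through the player's HealthComp, using a shared already-hit array to prevent repeat hits.
; The array is not cleared in this graph.
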(event `self.DoMeleeAttack`
  (`self.PlayAnimMontage` "/Game/Blueprint/Animation/Enemy/Melee/AM_AttackMelee.AM_AttackMelee" 1.0 (`KismetArrayLibrary.Array_Random` (`self.AttackSection`))))

(event `self.OnEnemyDead`
  (`SkeletalMeshComponent.PlayAnimation` (`self.Mesh`) "/Game/Blueprint/Animation/Enemy/Melee/MM_DeadAnim_DKF_Death.MM_DeadAnim_DKF_Death" false))

(event `self.AttackHitBox_R.OnComponentBeginOverlap`
  (params (OverlappedComponent :type "PrimitiveComponent Object Reference") (OtherActor :type "Actor Object Reference") (OtherComp :type "PrimitiveComponent Object Reference") (OtherBodyIndex :type Integer) (bFromSweep :type Boolean) (SweepResult :type "HitResult Structure (by ref)"))
  (bind _aireadyhitactors (`self.AIreadyHitActors`))
  (if (!= OtherActor self)
    (bind _asbp_player_character (cast `/Game/Blueprint/BP_PlayerCharacter` OtherActor))
    (if (not (`KismetArrayLibrary.Array_Contains` _aireadyhitactors))
      (`KismetArrayLibrary.Array_Add` _aireadyhitactors)
      (`HealthComponent.ApplyDamage` (`CharacterBased.HealthComp` _asbp_player_character) (`self.AttackDamage`) self))))

(event `self.AttackHitBox_L.OnComponentBeginOverlap`
  (params (OverlappedComponent :type "PrimitiveComponent Object Reference") (OtherActor :type "Actor Object Reference") (OtherComp :type "PrimitiveComponent Object Reference") (OtherBodyIndex :type Integer) (bFromSweep :type Boolean) (SweepResult :type "HitResult Structure (by ref)"))
  (bind _aireadyhitactors (`self.AIreadyHitActors`))
  (if (!= OtherActor self)
    (bind _asbp_player_character (cast `/Game/Blueprint/BP_PlayerCharacter` OtherActor))
    (if (not (`KismetArrayLibrary.Array_Contains` _aireadyhitactors OtherActor))
      (`KismetArrayLibrary.Array_Add` _aireadyhitactors OtherActor)
      (`HealthComponent.ApplyDamage` (`CharacterBased.HealthComp` _asbp_player_character) (`self.AttackDamage`) self))))

(fn `UserConstructionScript`
  (`parent.UserConstructionScript`))