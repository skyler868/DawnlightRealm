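; Final boss enemy Blueprint for a black dragon with claw, bite, fire breath and lightning ball attacks, each exposed as a montage-playing event.
; On BeginPlay it creates a boss HUD and binds its health bar to HealthComp; on death it plays the death animation and removes the HUD.
; Claw and bite hit volumes damage the player through HealthComp, using an already-hit actor list, not cleared here, to block repeat hits.
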(event `self.BP_PlayClaw`
  (`self.PlayAnimMontage` "/Game/Blueprint/Enemy/BossAnim/AM_Claw.AM_Claw" 1.0 "Attack"))

(event `self.BP_PlayBite`
  (`self.PlayAnimMontage` "/Game/Blueprint/Enemy/BossAnim/AM_Bite.AM_Bite" 1.0 "Attack"))

(event `self.BP_PlayFireBreath`
  (`self.PlayAnimMontage` "/Game/Blueprint/Enemy/BossAnim/AM_FireBreath.AM_FireBreath"))

(event `self.BP_PlayLightningBall`
  (`self.PlayAnimMontage` "/Game/Blueprint/Enemy/BossAnim/AM_LightningBall.AM_LightningBall"))

(event `self.OnEnemyDead`
  (`SkeletalMeshComponent.PlayAnimation` (`self.Mesh`) "/Game/BlackDragon/Animations/ANIM_BLACK_DRAGON_death.ANIM_BLACK_DRAGON_death" false)
  (`Widget.RemoveFromParent` (`self.HUDWidget`)))

(event `self.ReceiveBeginPlay`
  (bind _returnvalue (`|CreateWidget` "/Game/Blueprint/UI/Fight/WBP_BossHUD.WBP_BossHUD_C" null self))
  (set `self.HUDWidget` _returnvalue)
  (`UserWidget.AddToViewport` _returnvalue 0)
  (bind _healthcomp (`self.HealthComp`)
    (:`then`
      (set `/Game/Blueprint/UI/Fight/WBP_HealthBar.SelfHealthComp` _healthcomp (`/Game/Blueprint/UI/Fight/WBP_BossHUD.WBP_HealthBar` (`self.HUDWidget`))))
    (:`else`)))

(event `self.BiteHit.OnComponentBeginOverlap`
  (params (OverlappedComponent :type "PrimitiveComponent Object Reference") (OtherActor :type "Actor Object Reference") (OtherComp :type "PrimitiveComponent Object Reference") (OtherBodyIndex :type Integer) (bFromSweep :type Boolean) (SweepResult :type "HitResult Structure (by ref)"))
  (bind _aiready_hit_actors (`self.AIready Hit Actors`))
  (if (!= OtherActor self)
    (bind _asbp_player_character (cast `/Game/Blueprint/BP_PlayerCharacter` OtherActor))
    (if (not (`KismetArrayLibrary.Array_Contains` _aiready_hit_actors))
      (`KismetArrayLibrary.Array_Add` _aiready_hit_actors)
      (`HealthComponent.ApplyDamage` (`CharacterBased.HealthComp` _asbp_player_character) (`self.AttackDamage`) self))))

(event `self.ClawHit.OnComponentBeginOverlap`
  (params (OverlappedComponent :type "PrimitiveComponent Object Reference") (OtherActor :type "Actor Object Reference") (OtherComp :type "PrimitiveComponent Object Reference") (OtherBodyIndex :type Integer) (bFromSweep :type Boolean) (SweepResult :type "HitResult Structure (by ref)"))
  (bind _aiready_hit_actors (`self.AIready Hit Actors`))
  (if (!= OtherActor self)
    (bind _asbp_player_character (cast `/Game/Blueprint/BP_PlayerCharacter` OtherActor))
    (if (not (`KismetArrayLibrary.Array_Contains` _aiready_hit_actors))
      (`KismetArrayLibrary.Array_Add` _aiready_hit_actors)
      (`HealthComponent.ApplyDamage` (`CharacterBased.HealthComp` _asbp_player_character) (`self.AttackDamage`) self))))

(fn `UserConstructionScript`)