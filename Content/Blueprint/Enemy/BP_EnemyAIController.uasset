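; BP_EnemyAIController is an enemy AI controller that turns perception updates into Blackboard target state.
; When an actor tagged Player is successfully sensed, it stores that actor as TargetActor and sets HasTarget.
; Losing the player, or any perception update from an actor without that tag, clears both keys through a shared branch.
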(event `self.PerceptionComp.OnTargetPerceptionUpdated`
  (params (Actor :type "Actor Object Reference") (Stimulus :type "AIStimulus Structure"))
  (bind _blackboardcomp (`self.BlackboardComp`))
  (bind _blackboardcomp_2 (`self.BlackboardComp`))
  (if (`self.ActorHasTag` Actor "Player")
    (if (`.bSuccessfullySensed` (break `AIStimulus` Stimulus))
      (`BlackboardComponent.SetValueAsObject` _blackboardcomp_2 "TargetActor" Actor)
      (`BlackboardComponent.SetValueAsBool` _blackboardcomp_2 "HasTarget" true)
      (else
        (`BlackboardComponent.SetValueAsObject` _blackboardcomp "TargetActor" null :!label _label)
        (`BlackboardComponent.SetValueAsBool` _blackboardcomp "HasTarget" false)))
    (else
      (goto _label))))

(fn `UserConstructionScript`)