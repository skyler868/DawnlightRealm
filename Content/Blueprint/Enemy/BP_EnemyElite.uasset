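; Elite enemy Blueprint that fights with a spawned sword, which it equips on BeginPlay.
; DoEliteAttack measures distance to the blackboard TargetActor, playing a dash montage beyond DashMinRange, otherwise a weighted random combo or heavy attack.
; IsAttacking clears immediately after each montage starts, and GetRandomEliteAttack, which updates LastAttack from a pool, is not called here.
; On death it plays an animation, then unequips and drops the sword after a delay.
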(event `self.ReceiveBeginPlay`
  (`parent.ReceiveBeginPlay`)
  (bind _returnvalue (`|SpawnActorFromClass` "/Game/Blueprint/ItemActor/BP_Weapon_3.BP_Weapon_3_C" (`KismetMathLibrary.MakeTransform` (0.0 0.0 0.0)) "Undefined" "MultiplyWithRoot" null null))
  (bind _output_get (set `self.CurrentEquipSword` _returnvalue))
  (`WeaponBase.OnEquip` _output_get self))

(event `self.OnEnemyDead`
  (`SkeletalMeshComponent.PlayAnimation` (`self.Mesh`) "/Game/Blueprint/Animation/Enemy/Elite/MM_Dead_Dead_Anim.MM_Dead_Dead_Anim" false)
  (`KismetSystemLibrary.Delay` 1.0)
  (bind _currentequipsword (`self.CurrentEquipSword`)
    (:`then`
      (`WeaponBase.OnUnEquip` _currentequipsword)
      (`WeaponBase.DropToWorld` _currentequipsword))
    (:`else`)))

(event `self.DoEliteAttack`
  (if (not (`self.bIsAttacking`))
    (set `self.bIsAttacking` true)
    (bind _asbp_enemy_aicontroller (cast `/Game/Blueprint/Enemy/BP_EnemyAIController` (`self.GetController`)))
    (bind _blackboardcomp (`EnemyAIController.BlackboardComp` _asbp_enemy_aicontroller)
      (:`then`
        (bind _asactor (cast `Actor` (`BlackboardComponent.GetValueAsObject` _blackboardcomp "TargetActor")))
        (bind _output_get (set `self.TargetActor` _asactor))
        (bind _returnvalue (`self.ClacDistance` _output_get))
        (bind _output_get_2 (set `self.DistanceToTarget` _returnvalue))
        (if (> _output_get_2 (`self.DashMinRange`))
          ;[1 1 1] 远距离
          (`self.PlayAnimMontage` "/Game/Blueprint/Animation/Enemy/Elite/AM_Dash.AM_Dash" 1.0 "Default ")
          (set `self.bIsAttacking` false)
          (elif (< (`KismetMathLibrary.RandomInteger` 100) 65)
            (`self.PlayAnimMontage` "/Game/Blueprint/Animation/Enemy/Elite/AM_Combo.AM_Combo" 1.2 "Combo1")
            (set `self.bIsAttacking` false)
            (else
              (`self.PlayAnimMontage` "/Game/Blueprint/Animation/Enemy/Elite/AM_EHealviy.AM_EHealviy" 1.0 "Attack")
              (set `self.bIsAttacking` false)))))
      (:`else`))))

(fn `ClacDistance`
  (params (TargetActor :type "Actor Object Reference"))
  (returns (ReturnValue :type "Float (double-precision)"))
  (return (`KismetMathLibrary.VSize` (- (`self.K2_GetActorLocation` TargetActor) (`self.K2_GetActorLocation` self)))))

(fn `GetRandomEliteAttack`
  (bind _outitem (`KismetArrayLibrary.Array_Random` (`self.EliteAttackPool`)))
  (if (`|EnumEquality` (`self.LastAttack`) _outitem)
    (set `self.LastAttack` (`KismetArrayLibrary.Array_Random` (`self.EliteAttackPool`)))
    (return)
    (else
      (set `self.LastAttack` _outitem)
      (return))))

(fn `UserConstructionScript`
  (`parent.UserConstructionScript`))