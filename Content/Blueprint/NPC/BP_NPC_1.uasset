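; BP_NPC_1 is an NPC Blueprint that handles dialogue, quest rewards and quest notification popups for the player.
; ShowDialogue refreshes or creates the UWP_UIMain widget with the NPC as owner; on creation it pauses the game, switches to UI input and plays a voice greeting.
; EndDialogue closes the widget and restores gameplay, while GiveReward constructs reward items into the player's InventoryComponent.
; Separate events display quest receive and quest complete widgets.
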(event `self.ShowDialogue`
  (params (Node :type "DialogueNode Structure (by ref)"))
  (bind _returnvalue (`GameplayStatics.GetPlayerController` 0))
  (bind _dialoguewidget (`self.DialogueWidget`))
  (`/Engine/EditorBlueprintResources/StandardMacros.IsValid` _dialoguewidget
    (:`Is Valid`
      (`/Game/Blueprint/UI/UWP_UIMain.RefreshDialogue` _dialoguewidget Node))
    (:`Is Not Valid`
      (bind _returnvalue_2 (`|CreateWidget` "/Game/Blueprint/UI/UWP_UIMain.UWP_UIMain_C" null self))
      (bind _output_get (set `self.DialogueWidget` _returnvalue_2))
      (`/Game/Blueprint/UI/UWP_UIMain.RefreshDialogue` _output_get Node)
      (`UserWidget.AddToViewport` _output_get 0)
      (`WidgetBlueprintLibrary.SetInputMode_UIOnlyEx` _returnvalue null)
      (set `PlayerController.bShowMouseCursor` true _returnvalue)
      (`GameplayStatics.SetGamePaused` true)
      (`GameplayStatics.PlaySound2D` "/Game/Sound_Effects/VOICES/Female/VOICE_FEMALE_Hello_1_mono.VOICE_FEMALE_Hello_1_mono" 1.0 1.0 0.0 null null))))

(event `self.EndDialogue`
  (bind _returnvalue (`GameplayStatics.GetPlayerController` 0))
  (`/Game/Blueprint/UI/UWP_UIMain.CloseDialogue` (`self.DialogueWidget`))
  (set `self.DialogueWidget` null)
  (`WidgetBlueprintLibrary.SetInputMode_GameOnly` _returnvalue)
  (set `PlayerController.bShowMouseCursor` false _returnvalue)
  (`GameplayStatics.SetGamePaused` false))

(event `self.GiveReward`
  (params (reward :type "QuestReward Structure"))
  (for _array_element (`.RewardItems` (break `QuestReward` reward))
    (bind _asbp_player_character (cast `/Game/Blueprint/BP_PlayerCharacter` (`GameplayStatics.GetPlayerPawn` 0)))
    (bind _inventorycomponent (`PlayerCharacterBased.InventoryComponent` _asbp_player_character)
      (:`then`
        (bind _returnvalue (`|GenericCreateObject` _inventorycomponent _array_element))
        (`InventoryComponent.AddItem` _inventorycomponent _returnvalue))
      (:`else`))))

(event `self.ShowReceiveMessage`
  (bind _returnvalue (`|CreateWidget` "/Game/Blueprint/UI/Quest/UWP_QuestReceive.UWP_QuestReceive_C"))
  (`UserWidget.AddToViewport` _returnvalue 0))

(event `self.ShowSystemMessage`
  (bind _returnvalue (`|CreateWidget` "/Game/Blueprint/UI/Quest/UWP_QuestComplete.UWP_QuestComplete_C"))
  (`UserWidget.AddToViewport` _returnvalue 0))

(fn `UserConstructionScript`)