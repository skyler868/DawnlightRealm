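; Player controller that handles interaction input and owns the inventory, quest log, menu and interact prompt widgets.
; A forward sphere trace from the pawn finds actors implementing the Interactable interface, toggling the prompt every Tick and sending InteractMessage on the interact input.
; C, G and Z toggle inventory, quest log and menu, switching cursor and input mode.
; The quest log is created lazily from the character's QuestComponent; the other widgets are created at BeginPlay.
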(event `EnhancedInput|/Game/Input/Combat/IA_Interact`
  (params (ActionValue :type Boolean) (ElapsedSeconds :type "Float (double-precision)") (TriggeredSeconds :type "Float (double-precision)") (InputAction :type "InputAction Object Reference" :default "/Game/Input/Combat/IA_Interact.IA_Interact"))
  (:`Started`
    (bind (_hitactor _asbp_player_character _returnvalue) (`self.Check Interactable`))
    (if _returnvalue
      (message `Interactable.Interact` _hitactor _asbp_player_character))))

(event `self.ReceiveTick`
  (params (DeltaSeconds :type "Float (single-precision)"))
  (bind (_hitactor _asbp_player_character _returnvalue) (`self.Check Interactable`))
  (bind _interactui (`self.InteractUI`)
    (:`then`
      (if _returnvalue
        (`Widget.SetVisibility` _interactui "Visible")
        (else
          (`Widget.SetVisibility` _interactui "Hidden"))))
    (:`else`)))

(event `self.ReceiveBeginPlay`
  (bind _returnvalue (`|CreateWidget` "/Game/Blueprint/UI/Inventory/WBP_Inventroy.WBP_Inventroy_C"))
  (`UserWidget.AddToViewport` _returnvalue 0)
  (bind _output_get (set `self.InventroyRef` _returnvalue))
  (set `Widget.Visibility` "Collapsed" _output_get)
  (bind _returnvalue_2 (`|CreateWidget` "/Game/Blueprint/UI/WBP_Interact.WBP_Interact_C"))
  (`UserWidget.AddToViewport` _returnvalue_2 0)
  (set `Widget.Visibility` "Hidden" _returnvalue_2)
  (set `self.InteractUI` _returnvalue_2)
  (bind _returnvalue_3 (`|CreateWidget` "/Game/Blueprint/UI/WBP_MenuUI.WBP_MenuUI_C"))
  (`UserWidget.AddToViewport` _returnvalue_3 0)
  (bind _output_get_2 (set `self.MenuUI` _returnvalue_3))
  (set `Widget.Visibility` "Hidden" _output_get_2))

(event `Key|C`
  (params (Key :type "Key Structure"))
  (bind _returnvalue (`GameplayStatics.GetPlayerController` 0))
  (bind _inventroyref (`self.InventroyRef`))
  (:`Pressed`
    (`GameplayStatics.PlaySound2D` "/Engine/VREditor/Sounds/VR_grab.VR_grab" 1.0 1.0 0.0 null null)
    (bind _inventroyref_2 (`self.InventroyRef`)
      (:`then`
        (if (`|EnumEquality` (`Widget.Visibility` _inventroyref_2) "Visible")
          (`/Game/Blueprint/UI/Inventory/WBP_Inventroy.CloseInventory` (`self.InventroyRef`))
          (set `self.bShowMouseCursor` false)
          (`WidgetBlueprintLibrary.SetInputMode_GameOnly` _returnvalue)
          (else
            (`Widget.SetVisibility` _inventroyref "Visible")
            (`UserWidget.PlayAnimation` _inventroyref (`/Game/Blueprint/UI/Inventory/WBP_Inventroy.Start_End` _inventroyref) 0.0 1 "Forward" 1.0 false)
            (set `self.bShowMouseCursor` true)
            (`WidgetBlueprintLibrary.SetInputMode_GameAndUIEx` _returnvalue null "DoNotLock" false))))
      (:`else`))))

(event `Key|B`
  (params (Key :type "Key Structure")))

(event `Key|G`
  (params (Key :type "Key Structure"))
  (bind _returnvalue (`GameplayStatics.GetPlayerController` 0))
  (:`Pressed`
    (`GameplayStatics.PlaySound2D` "/Engine/VREditor/Sounds/VR_grab.VR_grab" 1.0 1.0 0.0 null null)
    (`/Engine/EditorBlueprintResources/StandardMacros.FlipFlop`
      (:`A`
        (bind _questlog (`self.QuestLog`)
          (:`then`
            (`UserWidget.PlayAnimation` _questlog (`/Game/Blueprint/UI/Quest/WBP_QuestLog.Fade` _questlog) 0.0 1 "Forward" 1.0 false)
            (`Widget.SetVisibility` _questlog "Visible")
            (set `self.bShowMouseCursor` true)
            (`WidgetBlueprintLibrary.SetInputMode_GameAndUIEx` _returnvalue null "DoNotLock" false))
          (:`else`
            (bind _asbp_player_character (cast `/Game/Blueprint/BP_PlayerCharacter` (`GameplayStatics.GetPlayerPawn` 0)))
            (bind _questcomponent (`PlayerCharacterBased.QuestComponent` _asbp_player_character)
              (:`then`
                (bind _returnvalue_2 (`|CreateWidget` "/Game/Blueprint/UI/Quest/WBP_QuestLog.WBP_QuestLog_C" null _questcomponent))
                (`UserWidget.PlayAnimation` _returnvalue_2 (`/Game/Blueprint/UI/Quest/WBP_QuestLog.Fade` _returnvalue_2) 0.0 1 "Forward" 1.0 false)
                (`UserWidget.AddToViewport` _returnvalue_2 0)
                (set `self.QuestLog` _returnvalue_2)
                (set `self.bShowMouseCursor` true)
                (`WidgetBlueprintLibrary.SetInputMode_GameAndUIEx` _returnvalue null "DoNotLock" false))
              (:`else`)))))
      (:`B`
        (bind _questlog_2 (`self.QuestLog`)
          (:`then`
            (`UserWidget.PlayAnimation` _questlog_2 (`/Game/Blueprint/UI/Quest/WBP_QuestLog.Fade` _questlog_2) 0.0 1 "Reverse" 1.0 false)
            (`KismetSystemLibrary.Delay` 0.3)
            (`Widget.SetVisibility` _questlog_2 "Collapsed")
            (set `self.bShowMouseCursor` false)
            (`WidgetBlueprintLibrary.SetInputMode_GameOnly` _returnvalue))
          (:`else`))))))

(event `Key|Z`
  (params (Key :type "Key Structure"))
  (:`Pressed`
    (`GameplayStatics.PlaySound2D` "/Engine/VREditor/Sounds/VR_grab.VR_grab" 1.0 1.0 0.0 null null)
    (bind _menuui (`self.MenuUI`)
      (:`then`
        (if (`Widget.IsVisible` _menuui)
          (`self.CloseMenuUI`)
          (else
            (`self.ShowMenuUI`))))
      (:`else`))))

(fn `Check Interactable`
  (returns (HitActor :type "Actor Object Reference") (`AsBP Player Character` :type "/Game/Blueprint/BP_PlayerCharacter Object Reference") (ReturnValue :type Boolean))
  (bind _asbp_player_character (cast `/Game/Blueprint/BP_PlayerCharacter` (`self.K2_GetPawn`))
    (:`then`
      (bind _rootcomponent (`Actor.RootComponent` _asbp_player_character))
      (bind _returnvalue (`SceneComponent.K2_GetComponentLocation` _rootcomponent))
      (bind _outhit (`KismetSystemLibrary.SphereTraceSingle` _returnvalue (+ _returnvalue (* (`SceneComponent.GetForwardVector` _rootcomponent) 400)) 100.0 "TraceTypeQuery3" false (`|MakeArray` _asbp_player_character :!type "Actor Object Reference")))
      (bind (_bblockinghit _binitialoverlap _time _distance _location _impactpoint _normal _impactnormal _physmat _hitactor) (`GameplayStatics.BreakHitResult` _outhit))
      (return _hitactor _asbp_player_character (`KismetSystemLibrary.DoesImplementInterface` _hitactor "/Script/DawnlightRealm.Interactable")))
    (:`CastFailed`
      (return null null false))))

(fn `CloseMenuUI`
  (set `Widget.Visibility` "Hidden" (`self.MenuUI`))
  (`WidgetBlueprintLibrary.SetInputMode_GameOnly` self)
  (set `self.bShowMouseCursor` false))

(fn `ShowMenuUI`
  (set `Widget.Visibility` "Visible" (`self.MenuUI`))
  (`WidgetBlueprintLibrary.SetInputMode_GameAndUIEx` self null)
  (set `self.bShowMouseCursor` true))

(fn `UserConstructionScript`)